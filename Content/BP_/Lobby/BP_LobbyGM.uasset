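; Lobby game mode that seats joining players as characters on display platforms, handles kicking and starts the match by server travel.
; BeginPlay orders platforms by index tags; a delay-polling macro holds login and logout updates until that finishes.
; Updates spawn characters on free platforms and clear departed players' platforms.
; Player info requests update the matching character, retry via the controller if unplaced, and refresh all-ready status on the first controller's UI.
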(event `self.ReceiveBeginPlay`
  (`self.SetupPlatforms`))

(event `self.K2_PostLogin`
  (params (NewPlayer :type "PlayerController Object Reference"))
  (`KismetArrayLibrary.Array_Add` (`self.PlayerControllers`) NewPlayer)
  (`self.IfPlatformIsDone` :!label _label
    (:`true`
      (`self.UpdatePlayerOnPlatforms`))))

(event `self.K2_OnLogout`
  (params (ExitingController :type "Controller Object Reference"))
  (bind _asplayer_controller (cast `PlayerController` ExitingController))
  (`KismetArrayLibrary.Array_RemoveItem` (`self.PlayerControllers`) _asplayer_controller)
  (goto _label))

(fn `CheckPlayersAreReady`
  (locals (PlayersReady :type Boolean))
  (set `local.PlayersReady` true)
  (for _array_element (`self.PlayerControllers`)
    (bind _asbp_lobby_pc (cast `/Game/BP_/Lobby/BP_LobbyPC` _array_element))
    (bind (_playerlobbyinfo_playercontroller _playerlobbyinfo_playername _playerlobbyinfo_bready) (break `/Game/BP_/Lobby/S_PlayerLobbyInfo` (`/Game/BP_/Lobby/BP_LobbyPC.PlayerLobbyInfo` _asbp_lobby_pc)))
    (if (not _playerlobbyinfo_bready)
      (set `local.PlayersReady` false)))
  (bind _asbp_lobby_pc_2 (cast `/Game/BP_/Lobby/BP_LobbyPC` (`GameplayStatics.GetPlayerController` 0)))
  (set `/Game/BP_/Lobby/Widgets/WB_LobbyUI.PlayersAreReady` (`local.PlayersReady`) (`/Game/BP_/Lobby/BP_LobbyPC.LobbyUI` _asbp_lobby_pc_2)))

(fn `KickPlayer`
  (params (PlayerToKick :type "PlayerController Object Reference"))
  (`AdvancedSessionsLibrary.KickPlayer` PlayerToKick))

(fn `SetupPlatforms`
  (bind _outactors (`GameplayStatics.GetAllActorsOfClass` "/Game/BP_/Lobby/BP_LobbyPlayerPlatform.BP_LobbyPlayerPlatform_C"))
  (for _index (range (+ (`KismetArrayLibrary.Array_LastIndex` _outactors) 1))
    (bind _outactors_2 (`GameplayStatics.GetAllActorsOfClassWithTag` "/Game/BP_/Lobby/BP_LobbyPlayerPlatform.BP_LobbyPlayerPlatform_C" (`KismetStringLibrary.Conv_StringToName` (`KismetStringLibrary.Conv_IntToString` _index))))
    (`KismetArrayLibrary.Array_Add` (`self.PlayerPlatforms`) (`|GetArrayItem` _outactors_2)))
  (set `self.SetupPlatformsDone` true))

(fn `StartMatch`
  (params (Map :type String))
  (`AdvancedSessionsLibrary.ServerTravel` Map)
  (for _array_element (`self.PlayerControllers`)
    (bind _asbp_lobby_pc (cast `/Game/BP_/Lobby/BP_LobbyPC` _array_element))
    (`/Game/BP_/Lobby/BP_LobbyPC.StartMatch` _asbp_lobby_pc)))

(fn `UpdatePlayerLobbyInfo`
  (params (RequestingPC :type "PlayerController Object Reference"))
  (locals (PlayerController :type "PlayerController Object Reference"))
  (bind (_playerlobbyinfo_playercontroller _playerlobbyinfo_playername _playerlobbyinfo_bready) (break `/Game/BP_/Lobby/S_PlayerLobbyInfo` (`/Game/BP_/Lobby/BP_LobbyPC.PlayerLobbyInfo` (cast `/Game/BP_/Lobby/BP_LobbyPC` (`local.RequestingPC`) :!pure true))))
  (set `local.PlayerController` RequestingPC)
  (for _array_element (`self.PlayerPlatforms`)
    (if (== (`/Game/BP_/Lobby/BP_LobbyPlayerPlatform.PlayerController` _array_element) (`local.PlayerController`))
      (bind _asbp_player_lobby (cast `/Game/BP_/Game/Player/BP_PlayerLobby` (`/Game/BP_/Lobby/BP_LobbyPlayerPlatform.CurrentCharacter` _array_element)))
      (`/Game/BP_/Game/Player/BP_PlayerLobby.UpdateLobbyInfo` _asbp_player_lobby (make `/Game/BP_/Lobby/S_PlayerLobbyInfo` (`local.RequestingPC`) (`KismetTextLibrary.Conv_StringToText` (`AdvancedSessionsLibrary.GetPlayerName` (`local.RequestingPC`))) _playerlobbyinfo_bready (`Controller.PlayerState` (`local.RequestingPC`))))
      (`self.CheckPlayersAreReady`)
      (return)))
  (`/Game/BP_/Lobby/BP_LobbyPC.RetryUpdateLobbyInfo` (cast `/Game/BP_/Lobby/BP_LobbyPC` (`local.RequestingPC`) :!pure true)))

(fn `UpdatePlayerOnPlatforms`
  (locals (Loop :type Boolean) (Controller :type "PlayerController Object Reference"))
  (for _array_element (`self.PlayerControllers`)
    (set `local.Controller` _array_element)
    (set `local.Loop` false)
    (for _array_element_2 (`self.PlayerPlatforms`)
      (if (== (`/Game/BP_/Lobby/BP_LobbyPlayerPlatform.PlayerController` _array_element_2) (`local.Controller`))
        (set `local.Loop` true)
        (break)))
    (if (not (`local.Loop`))
      (for _array_element_3 (`self.PlayerPlatforms`)
        (`/Engine/EditorBlueprintResources/StandardMacros.IsValid` (`/Game/BP_/Lobby/BP_LobbyPlayerPlatform.PlayerController` _array_element_3)
          (:`Is Not Valid`
            (`/Game/BP_/Lobby/BP_LobbyPlayerPlatform.SpawnCharacter` _array_element_3 (`local.Controller`))
            (break))))))
  (for _array_element_4 (`self.PlayerPlatforms`)
    (if (not (`KismetArrayLibrary.Array_Contains` (`self.PlayerControllers`) (`/Game/BP_/Lobby/BP_LobbyPlayerPlatform.PlayerController` _array_element_4)))
      (`/Game/BP_/Lobby/BP_LobbyPlayerPlatform.Clear` _array_element_4))))

(fn `UserConstructionScript`)