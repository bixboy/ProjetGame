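; BP_LobbyPlayerPlatform is a lobby slot that shows a player's character or an open-friend-list widget when empty.
; On BeginPlay, the server links the widget to the platform and makes it visible.
; SpawnCharacter replaces any existing BP_PlayerLobby at the spawn transform and hides the widget, while Clear destroys it and restores the widget.
; ShowFriendList collapses the button widget and opens the passed friend list for this platform.
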(event `self.ReceiveBeginPlay`
  (`self.SetupServer`))

(event `SpawnCharacter`
  (params (PlayerController :type "PlayerController Object Reference"))
  (bind _currentcharacter (`self.CurrentCharacter`))
  (set `self.PlayerController` PlayerController)
  (`/Engine/EditorBlueprintResources/StandardMacros.IsValid` _currentcharacter
    (:`Is Valid`
      (`self.K2_DestroyActor` _currentcharacter))
    (:`Is Not Valid`
      _))
  (bind _returnvalue (`|SpawnActorFromClass` "/Game/BP_/Game/Player/BP_PlayerLobby.BP_PlayerLobby_C" (`SceneComponent.K2_GetComponentToWorld` (`self.PlayerSpawnTransform`)) "AlwaysSpawn" "MultiplyWithRoot" null null))
  (set `self.CurrentCharacter` _returnvalue)
  (`SceneComponent.SetVisibility` (`self.OpenFriendList`) false false))

(event `Clear`
  (bind _currentcharacter (`self.CurrentCharacter`))
  (set `self.PlayerController` null)
  (`/Engine/EditorBlueprintResources/StandardMacros.IsValid` _currentcharacter
    (:`Is Valid`
      (`self.K2_DestroyActor` _currentcharacter)
      (set `self.CurrentCharacter` null))
    (:`Is Not Valid`
      _))
  (`SceneComponent.SetVisibility` (`self.OpenFriendList`) true false))

(fn `SetupServer`
  (if (`KismetSystemLibrary.IsServer`)
    (bind _aswb_open_friend_list (cast `/Game/BP_/Lobby/Widgets/WB_OpenFriendList` (`WidgetComponent.GetWidget` (`self.OpenFriendList`))))
    (set `/Game/BP_/Lobby/Widgets/WB_OpenFriendList.PlatformRef` self _aswb_open_friend_list)
    (`SceneComponent.SetVisibility` (`self.OpenFriendList`) true false)))

(fn `ShowFriendList`
  (params (Show :type Boolean) (FriendList :type "/Game/BP_/Lobby/Widgets/WB_LobbyUI Object Reference"))
  (if Show
    (`Widget.SetVisibility` (`WidgetComponent.GetWidget` (`self.OpenFriendList`)) "Collapsed")
    (`/Game/BP_/Lobby/Widgets/WB_LobbyUI.ShowFriendList` (`local.FriendList`) true self)
    (else
      (`Widget.SetVisibility` (`WidgetComponent.GetWidget` (`self.OpenFriendList`)) "Visible"))))

(fn `UserConstructionScript`)