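; BPC_XP is a player component that tracks XP and level, loading both from the game instance's save at BeginPlay.
; XP gains pass from a server event to a client event, applying only on the locally controlled player.
; Reaching MaxXP raises the level, resets XP without carrying overflow and refreshes the threshold via MaxXpInCrease, whose level-curve formula appears unconnected.
; Each change is saved through the game instance and printed.
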(event `self.ReceiveBeginPlay`
  (bind _save (message `/Game/BP_/Interface/BPI_Saving.GetSave` (`GameplayStatics.GetGameInstance`)))
  (bind (_playerinfo_playercontroller _playerinfo_playername _playerinfo_playerstate _playerinfo_xp _playerinfo_level) (break `/Game/BP_/MainMenu/S_MainPlayerInfo` (`/Game/BP_/Saves/BP_PlayerDataSave.PlayerInfo` _save)))
  (set `self.CurrentXP` _playerinfo_xp)
  (set `self.Level` _playerinfo_level)
  (set `self.MaxXP` (`self.MaxXpInCrease`))
  (bind _asbp_player (cast `/Game/BP_/Game/Player/BP_Player` (`self.GetOwner`)))
  (set `self.OwnerPlayer` _asbp_player))

(event `IncreaseXpServer`
  (params (AddXp :type Integer))
  (`self.IncreaseXpClient` AddXp))

(event `IncreaseXpClient`
  (params (AddedXP :type Integer))
  (`self.IncreaseXP` AddedXP))

(fn `IncreaseLevel`
  (params (AddedLevel :type Integer))
  (set `self.Level` (+ (`self.Level`) AddedLevel))
  (set `self.MaxXP` (`self.MaxXpInCrease`))
  (set `self.CurrentXP` 0)
  (`self.UpdateSave`))

(fn `IncreaseXP`
  (params (AddedXP :type Integer))
  (if (`Pawn.IsLocallyControlled` (`self.OwnerPlayer`))
    (set `self.CurrentXP` (+ AddedXP (`self.CurrentXP`)))
    (if (>= (`self.CurrentXP`) (`self.MaxXP`))
      (`self.IncreaseLevel` 1)
      (`KismetSystemLibrary.PrintString` "Level Passed")
      (else
        (`self.UpdateSave`)))))

(fn `UpdateSave`
  (bind _save (message `/Game/BP_/Interface/BPI_Saving.GetSave` (`GameplayStatics.GetGameInstance`)))
  (bind _structout (setmembers `/Game/BP_/MainMenu/S_MainPlayerInfo` :`StructRef` (`/Game/BP_/Saves/BP_PlayerDataSave.PlayerInfo` _save) :`XP` (`self.CurrentXP`) :`Level` (`self.Level`)))
  (message `/Game/BP_/Interface/BPI_Saving.Save` (`GameplayStatics.GetGameInstance`) _structout)
  (bind _save_2 (message `/Game/BP_/Interface/BPI_Saving.GetSave` (`GameplayStatics.GetGameInstance`)))
  (bind (_playerinfo_playercontroller _playerinfo_playername _playerinfo_playerstate _playerinfo_xp _playerinfo_level) (break `/Game/BP_/MainMenu/S_MainPlayerInfo` (`/Game/BP_/Saves/BP_PlayerDataSave.PlayerInfo` _save_2)))
  (`KismetSystemLibrary.PrintString` (`KismetStringLibrary.Concat_StrStr` "Current XP : " (`KismetStringLibrary.Conv_IntToString` _playerinfo_xp) " / Need XP : " (`KismetStringLibrary.Conv_IntToString` (`self.MaxXP`)) " / Your Level : " (`KismetStringLibrary.Conv_IntToString` _playerinfo_level))))