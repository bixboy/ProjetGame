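; Actor component that lets its owner vault over obstacles ahead with a motion-warped montage.
; A forward sphere trace finds the obstacle, then stepped line traces measure its top edge, depth and landing point, with debug drawing.
; The obstacle-top midpoint and landing point become two warp targets before the montage plays in Flying mode with capsule collision off.
; ResetVault restores Falling movement and collision and clears the Busy guard.
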(event `VaultOverObject`
  (set `self.Busy` true)
  (`CharacterMovementComponent.SetMovementMode` (`self.Character Movement`) "MOVE_Flying" 0)
  (`PrimitiveComponent.SetCollisionEnabled` (`self.Capsule Collider`) "NoCollision")
  (`|PlayMontage` (`self.Skeletal Mesh`) (`self.VaultAnim`)))

(event `ResetVault`
  (set `self.Busy` false)
  (`CharacterMovementComponent.SetMovementMode` (`self.Character Movement`) "MOVE_Falling" 0)
  (`PrimitiveComponent.SetCollisionEnabled` (`self.Capsule Collider`) "QueryAndPhysics"))

(fn `GetInitialObjectLocation`
  (locals (InitialImpactLocation :type "Vector Structure"))
  (bind _returnvalue (`self.GetOwner`))
  (bind _returnvalue_2 (- (`Actor.K2_GetActorLocation` _returnvalue) (0.0 0.0 50.0)))
  (if (not (`self.Busy`))
    (bind (_outhit _returnvalue_3) (`KismetSystemLibrary.SphereTraceSingle` :`Start` _returnvalue_2 :`End` (+ _returnvalue_2 (* (`KismetMathLibrary.GetForwardVector` (`Actor.K2_GetActorRotation` _returnvalue)) 250.0)) :`Radius` 10.0 :`TraceChannel` "TraceTypeQuery1" :`DrawDebugType` "ForDuration"))
    (if _returnvalue_3
      (bind _output_get (set `local.InitialImpactLocation` (`.ImpactPoint` (`GameplayStatics.BreakHitResult` _outhit))))
      (`self.GetObjectDimensions` _output_get)
      (else
        (set `local.InitialImpactLocation` (0.0 0.0 0.0))))))

(fn `GetObjectDimensions`
  (params (InitialImpactLocation :type "Vector Structure"))
  (locals (InitialImpactVector :type "Vector Structure") (ObjectHeightIndex :type Integer) (ObjectDepthIndex :type Integer))
  (bind (_returnvalue_x _returnvalue_y _returnvalue_z) (`KismetMathLibrary.BreakVector` (* (`local.ObjectHeightIndex`) 5)))
  (bind _returnvalue (+ (`KismetMathLibrary.MakeVector` 0.0 0.0 _returnvalue_z) (- (`local.InitialImpactVector`) (0.0 0.0 30.0))))
  (bind _returnvalue_2 (+ (`self.ObjectDepthVector`) (* (`KismetMathLibrary.GetForwardVector` (`Actor.K2_GetActorRotation` (`self.GetOwner`))) 150.0)))
  (bind _returnvalue_3 (+ (+ (`self.ObjectHeightVector`) (0.0 0.0 30.0)) (* (`KismetMathLibrary.GetForwardVector` (`Actor.K2_GetActorRotation` (`self.GetOwner`))) (* (`local.ObjectDepthIndex`) 5))))
  (set `local.InitialImpactVector` InitialImpactLocation)
  (for _index (range 1 51)
    (set `local.ObjectHeightIndex` _index)
    (bind (_outhit _returnvalue_4) (`KismetSystemLibrary.LineTraceSingle` :`Start` _returnvalue :`End` (+ _returnvalue (* (`KismetMathLibrary.GetForwardVector` (`Actor.K2_GetActorRotation` (`self.GetOwner`))) 75.0)) :`TraceChannel` "TraceTypeQuery1" :`DrawDebugType` "ForDuration"))
    (if _returnvalue_4
      (set `self.ObjectHeightVector` (`.ImpactPoint` (`GameplayStatics.BreakHitResult` _outhit)))
      (else
        (break))))
  (for _index_2 (range 1 51)
    (set `local.ObjectDepthIndex` _index_2)
    (bind (_outhit_2 _returnvalue_5) (`KismetSystemLibrary.LineTraceSingle` :`Start` _returnvalue_3 :`End` (- _returnvalue_3 (0.0 0.0 50.0)) :`TraceChannel` "TraceTypeQuery1" :`DrawDebugType` "ForDuration"))
    (if _returnvalue_5
      (set `self.ObjectDepthVector` (`.ImpactPoint` (`GameplayStatics.BreakHitResult` _outhit_2)))
      (else
        (break))))
  (bind (_outhit_3 _returnvalue_6) (`KismetSystemLibrary.LineTraceSingle` :`Start` _returnvalue_2 :`End` (- _returnvalue_2 (0.0 0.0 150.0)) :`TraceChannel` "TraceTypeQuery1" :`DrawDebugType` "ForDuration"))
  (if _returnvalue_6
    (bind (_bblockinghit _binitialoverlap _time _distance _location _impactpoint _normal _impactnormal _physmat _hitactor _hitcomponent _hitbonename _bonename _hititem _elementindex _faceindex _tracestart _traceend) (`GameplayStatics.BreakHitResult` _outhit_3))
    (set `self.LandingVector` _impactpoint)
    (else
      (set `self.LandingVector` (+ _traceend (0.0 0.0 50.0)))))
  (`KismetSystemLibrary.DrawDebugSphere` (`self.ObjectHeightVector`) 20.0 12 (struct :`R` 1.0 :`G` 1.0 :`B` 1.0 :`A` 1.0) 5.0)
  (`KismetSystemLibrary.DrawDebugSphere` (`self.ObjectDepthVector`) 20.0 12 (struct :`R` 1.0 :`B` 0.190898 :`A` 1.0) 5.0)
  (`KismetSystemLibrary.DrawDebugSphere` (`self.LandingVector`) 20.0 12 (struct :`R` 0.005214 :`B` 1.0 :`A` 1.0) 5.0)
  (`self.SetMotionWarpPosition`))

(fn `SetMotionWarpPosition`
  (`MotionWarpingComponent.AddOrUpdateWarpTarget` (`self.MotionWarping`) (make `MotionWarpingTarget` "Warp1" (`KismetMathLibrary.VLerp` (`self.ObjectHeightVector`) (`self.ObjectDepthVector`) 0.5) (`Actor.K2_GetActorRotation` (`self.GetOwner`)) null "None" false))
  (`MotionWarpingComponent.AddOrUpdateWarpTarget` (`self.MotionWarping`) (make `MotionWarpingTarget` "Warp2" (`self.LandingVector`) (`Actor.K2_GetActorRotation` (`self.GetOwner`)) null "None"))
  (`self.VaultOverObject`))