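; BPC_Score is a component on BP_Player that keeps the player's score.
; AddScore awards one fixed value by priority of kill, headshot, then hit, while SubstractScore deducts a supplied amount.
; Server-named events forward to client-named events, which update the score and, only for a locally controlled owner, pass the change to the player's MainHUD.
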(event `self.ReceiveBeginPlay`
  (bind _asbp_player (cast `/Game/BP_/Player/BP_Player` (`self.GetOwner`)))
  (set `self.OwnerPlayer` _asbp_player))

(event `AddScoreServer`
  (params (Dead :type Boolean) (Head :type Boolean) (Hit :type Boolean))
  (`self.AddScoreClient` Dead Head Hit))

(event `AddScoreClient`
  (params (Dead :type Boolean) (Head :type Boolean) (Hit :type Boolean))
  (bind _valuereturn (`self.AddScore` Dead Head Hit))
  (if (`Pawn.IsLocallyControlled` (`self.OwnerPlayer`))
    (`/Game/BP_/Widgets/WB_MainHUD.AddScore` (`/Game/BP_/Player/BP_Player.MainHUD` (`self.OwnerPlayer`)) _valuereturn)))

(event `SubstractServer`
  (params (Value :type Integer))
  (`self.SubstractClient` Value))

(event `SubstractClient`
  (params (Value :type Integer))
  (bind _valuereturn (`self.SubstractScore` Value))
  (if (`Pawn.IsLocallyControlled` (`self.OwnerPlayer`))
    (`/Game/BP_/Widgets/WB_MainHUD.SubstractScore` (`/Game/BP_/Player/BP_Player.MainHUD` (`self.OwnerPlayer`)) _valuereturn)))

(fn `AddScore`
  (params (Dead :type Boolean) (Head :type Boolean) (Hit :type Boolean))
  (returns (ValueReturn :type Integer))
  (locals (Value :type Integer))
  (if Dead
    (set `local.Value` 50)
    (set `self.Score` (+ (`local.Value`) (`self.Score`)) :!label _label)
    (return (`local.Value`))
    (elif Head
      (set `local.Value` 15)
      (goto _label)
      (elif Hit
        (set `local.Value` 10)
        (goto _label)))))

(fn `SubstractScore`
  (params (Value :type Integer))
  (returns (ValueReturn :type Integer))
  (set `self.Score` (- (`self.Score`) (`local.Value`)))
  (return (`local.Value`)))