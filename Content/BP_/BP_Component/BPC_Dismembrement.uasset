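; Actor component that adds bone-based dismemberment to its owner's skeletal mesh.
; RenameBones folds hip, upper spine, neck and head hits into Spine, then subtracts damage from that bone's entry in a breakable-bone health map.
; At zero health, Dismemberment breaks the constraint with a randomized impulse, hides the bone and attaches particle emitters.
; It also records broken bones and traces downward to place a temporary ground decal.
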(event `self.ReceiveBeginPlay`
  (set `self.SkeletalMesh` (`Actor.GetComponentByClass` (`self.GetOwner`) "/Script/Engine.SkeletalMeshComponent")))

(fn `ApplyDamageToBone`
  (returns (BoneIsBreak :type Boolean))
  (bind (_value _returnvalue) (`BlueprintMapLibrary.Map_Find` (`self.BreakableBones`) (`self.HitBone`)))
  (if _returnvalue
    (`BlueprintMapLibrary.Map_Add` (`self.BreakableBones`) (`self.HitBone`) (- _value (`self.AppliedDamage`)))
    (return (<= (`BlueprintMapLibrary.Map_Find` (`self.BreakableBones`) (`self.HitBone`)) 0))))

(fn `Dismemberment`
  (bind _hitbone (`self.HitBone`))
  (bind _skeletalmesh (`self.SkeletalMesh`))
  (bind (_returnvalue_location _returnvalue_rotation) (`KismetMathLibrary.BreakTransform` (`SceneComponent.GetSocketTransform` (`self.SkeletalMesh`) (`self.HitBone`) "RTS_World")))
  (bind _returnvalue (`SceneComponent.K2_GetComponentLocation` (`self.SkeletalMesh`)))
  (bind (_returnvalue_location_2 _returnvalue_rotation_2) (`KismetMathLibrary.BreakTransform` (`SceneComponent.GetSocketTransform` (`self.SkeletalMesh`) (`self.HitBone`) "RTS_World")))
  (bind (_returnvalue_location_3 _returnvalue_rotation_3) (`KismetMathLibrary.BreakTransform` (`SceneComponent.GetSocketTransform` (`self.SkeletalMesh`) (`self.HitBone`) "RTS_World")))
  (`SkeletalMeshComponent.BreakConstraint` _skeletalmesh (`self.CalculateImpulse`) (`self.GetSocketLocation`) _hitbone)
  (`SkinnedMeshComponent.HideBoneByName` _skeletalmesh _hitbone "PBO_None")
  (`GameplayStatics.SpawnEmitterAttached` null (`self.SkeletalMesh`) (`self.HitBone`) _returnvalue_location_3 _returnvalue_rotation_3 (2.0 2.0 2.0))
  (`GameplayStatics.SpawnEmitterAttached` null (`self.SkeletalMesh`) (`self.HitBone`) _returnvalue_location _returnvalue_rotation)
  (`GameplayStatics.SpawnEmitterAttached` null (`self.SkeletalMesh`) (`self.HitBone`) _returnvalue_location_2 _returnvalue_rotation_2)
  (set `self.HasSpineBroken` (== (`self.HitBone`) "Spine"))
  (`KismetArrayLibrary.Array_Add` (`self.BrokenBones`) (`self.HitBone`))
  (bind _outhit (`KismetSystemLibrary.LineTraceSingle` _returnvalue (+ _returnvalue (* (0.0 0.0 -1.0) 1000.0)) "TraceTypeQuery1"))
  (bind (_bblockinghit _binitialoverlap _time _distance _location _impactpoint _normal) (`GameplayStatics.BreakHitResult` _outhit))
  (`GameplayStatics.SpawnDecalAtLocation` null (-63.0 -128.0 -128.0) _location (`KismetMathLibrary.Conv_VectorToRotator` _normal) 60.0))

(fn `renameBones`
  (params (HitBone :type Name) (ImpactPoint :type "Vector Structure"))
  (bind _output_get (set `self.HitBone` HitBone))
  (set `self.ImpactPoint` ImpactPoint)
  (switch `name` _output_get
    (:`Default`
      _)
    (:`Hips`
      (set `self.HitBone` "Spine" :!label _label))
    (:`Spine1`
      (goto _label))
    (:`Spine2`
      (goto _label))
    (:`Neck`
      (goto _label))
    (:`Head`
      (goto _label)))
  (bind _boneisbreak (`self.ApplyDamageToBone`))
  (if _boneisbreak
    (`self.Dismemberment`)))