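; BPC_Health is an actor component that tracks health, damage and death for its owner.
; TakeDamage applies clamped damage, doubles it for headshots or kills instantly, and calls Death when health runs out.
; Death flags the owner dead, passes impulse point, hit bone and killer through DeathMessage, and prints the saved player name.
; UpdateHealth sets a new maximum and refills health, while Revive restores it only with the revive perk.
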(event `self.ReceiveBeginPlay`
  (`self.SetHealth`))

(fn `Death`
  (params (ImpulsePoint :type "Vector Structure") (BoneHit :type Name) (DamageCauser :type "/Game/BP_/Game/Player/BP_Player Object Reference"))
  (set `self.IsDead` true)
  (message `/Game/BP_/Interface/BPI_Health.Death` (`self.GetOwner`) (`local.ImpulsePoint`) (`local.BoneHit`) (`local.DamageCauser`))
  (bind _save (message `/Game/BP_/Interface/BPI_Saving.GetSave` (`GameplayStatics.GetGameInstance`)))
  (bind (_playerinfo_playercontroller _playerinfo_playername) (break `/Game/BP_/MainMenu/S_MainPlayerInfo` (`/Game/BP_/Saves/BP_PlayerDataSave.PlayerInfo` _save)))
  (`KismetSystemLibrary.PrintString` (`KismetStringLibrary.Concat_StrStr` (`KismetTextLibrary.Conv_TextToString` _playerinfo_playername) " : " "Is Dead")))

(fn `Revive`
  (if (`self.CanRevivePerk`)
    (set `self.IsDead` false)
    (`self.SetHealth`)))

(fn `SetHealth`
  (set `self.CurrentHealth` (`self.MaxHealth`)))

(fn `TakeDamage`
  (params (Instigator :type "/Game/BP_/Game/Player/BP_Player Object Reference") (InstantKill :type Boolean) (HeadShot :type Boolean) (Damage :type "Float (double-precision)") (ImpactPoint :type "Vector Structure") (BoneHit :type Name))
  (locals (DamageCauser :type "/Game/BP_/Game/Player/BP_Player Object Reference"))
  (set `local.DamageCauser` Instigator)
  (if (not (`self.IsDead`))
    (if (`local.InstantKill`)
      (set `self.CurrentHealth` 0.0)
      (`self.Death` (`local.ImpactPoint`) (`local.BoneHit`) (`local.DamageCauser`))
      (else
        (if (`local.HeadShot`)
          (set `self.CurrentHealth` (`KismetMathLibrary.FClamp` (- (`self.CurrentHealth`) (* (`local.Damage`) 2.0)) 0.0 (`self.MaxHealth`)))
          (else
            (set `self.CurrentHealth` (`KismetMathLibrary.FClamp` (- (`self.CurrentHealth`) (`local.Damage`)) 0.0 (`self.MaxHealth`)))))
        (if (<= (`self.CurrentHealth`) 0.0)
          (`self.Death` (`local.ImpactPoint`) (`local.BoneHit`) (`local.DamageCauser`)))))))

(fn `UpdateHealth`
  (params (NewHealth :type "Float (double-precision)"))
  (set `self.MaxHealth` NewHealth)
  (`self.SetHealth`))