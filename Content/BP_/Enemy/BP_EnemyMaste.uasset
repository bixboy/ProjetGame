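; Base enemy Blueprint that handles health, damage intake and death.
; On BeginPlay it creates its health component through AddBPCHealth using its Health value and keeps a reference to it.
; TakeDamage forwards damage and the instant-kill flag to that component, always with headshot off, and the Death event destroys the actor.
; Attack is a stub that returns zero.
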(event `self.ReceiveBeginPlay`
  (`self.SetupEnemy`))

(event `/Game/BP_/Interface/BPI_Health.TakeDamage`
  (params (InstantKill :type Boolean) (Damage :type "Float (double-precision)"))
  (`/Game/BP_/BP_Component/BPC_Health.TakeDamage` (`self.HealthComponent`) InstantKill false Damage))

(event `/Game/BP_/Interface/BPI_Health.Death`
  (`self.K2_DestroyActor`))

(fn `Attack`
  (returns (AnimDuration :type "Float (double-precision)"))
  (return 0.0))

(fn `SetupEnemy`
  (bind _returnvalue (`AddComponent|NODE_AddBPC_Health-0` :`MaxHealth` (`self.Health`)))
  (set `self.HealthComponent` _returnvalue))

(fn `UserConstructionScript`)