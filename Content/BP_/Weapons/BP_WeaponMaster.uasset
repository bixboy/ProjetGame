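; BP_WeaponMaster is a weapon that a BP_Player picks up by overlapping its sphere, then fires.
; Overlap stores the player and chains AttachServeur and AttachClient events into AttachWeapon, which snaps it to the first-person mesh when locally controlled, otherwise the third-person body.
; Fire spawns a projectile at the Ammo socket, offset and aimed by player zero's camera, then plays sound and a first-person shoot montage.
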(event `self.SphereCollision.OnComponentBeginOverlap`
  (params (OverlappedComponent :type "PrimitiveComponent Object Reference") (OtherActor :type "Actor Object Reference") (OtherComp :type "PrimitiveComponent Object Reference") (OtherBodyIndex :type Integer) (bFromSweep :type Boolean) (SweepResult :type "HitResult Structure (by ref)"))
  (if (== (`GameplayStatics.GetObjectClass` OtherActor) "/Game/BP_/Player/BP_Player.BP_Player_C")
    (bind _asbp_player (cast `/Game/BP_/Player/BP_Player` OtherActor))
    (set `self.PlayerRef` _asbp_player)
    (`self.AttachServeur`)))

(event `AttachServeur`
  (`self.AttachClient`))

(event `AttachClient`
  (`self.AttachWeapon`))

(event `/Game/BP_/Interface/BPI_Weapon.Fire`
  (bind _returnvalue (`PlayerCameraManager.GetCameraRotation` (`GameplayStatics.GetPlayerCameraManager` 0)))
  (bind _returnvalue_2 (+ (`SceneComponent.GetSocketLocation` (`self.SkeletalMesh`) "Ammo") (`KismetMathLibrary.GreaterGreater_VectorRotator` (`self.ProjectileOffset`) _returnvalue)))
  (`|SpawnActorFromClass` "/Game/BP_/Weapons/BP_ProjectileMaster.BP_ProjectileMaster_C" (`KismetMathLibrary.MakeTransform` _returnvalue_2 _returnvalue) "Undefined" "OverrideRootScale" null 0 null)
  (`GameplayStatics.PlaySoundAtLocation` (`self.SoundFire`) _returnvalue_2 (struct) 1.0 1.0 0.0 null null null null)
  (`AnimInstance.Montage_Play` (`SkeletalMeshComponent.GetAnimInstance` (`/Game/BP_/Player/BP_Player.FirstPersonMesh` (`self.PlayerRef`))) "/Game/Animations/PlayerAnim/Animations/FP_Rifle_Shoot_Montage.FP_Rifle_Shoot_Montage" 1.0 "MontageLength" 0.0 true))

(fn `AttachWeapon`
  (bind _playerref (`self.PlayerRef`))
  (set `/Game/BP_/Player/BP_Player.Weapon` self _playerref)
  (if (`Pawn.IsLocallyControlled` _playerref)
    (`self.K2_AttachToComponent` (`/Game/BP_/Player/BP_Player.FirstPersonMesh` _playerref) "GripPoint" "SnapToTarget" "SnapToTarget" "SnapToTarget")
    (else
      (`self.K2_AttachToComponent` (`/Game/BP_/Player/BP_Player.TP_Body` (`self.PlayerRef`)) "GripWeapon" "SnapToTarget" "SnapToTarget" "SnapToTarget")))
  (set `/Game/BP_/Player/BP_Player.bHasRifle` true (`self.PlayerRef`)))

(fn `UserConstructionScript`)