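; Base grenade projectile Blueprint that is thrown from an attached parent and explodes on a timed fuse.
; The fuse runs from BeginPlay, independent of the throw, and ends in Explod, which spawns particles and sound, fires a radial impulse and destroys the actor.
; Throw runs once, detaching the grenade, launching it through ProjectileMovement and enabling collision after a short delay.
; The hit event is empty and the bounce sound is unconnected.
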(event `self.ReceiveBeginPlay`
  (`KismetSystemLibrary.Delay` (`self.DurationGrenade`))
  (`self.Explod`))

(event `self.Grenade.OnComponentHit`
  (params (HitComponent :type "PrimitiveComponent Object Reference") (OtherActor :type "Actor Object Reference") (OtherComp :type "PrimitiveComponent Object Reference") (NormalImpulse :type "Vector Structure") (Hit :type "HitResult Structure (by ref)")))

(event `Throw`
  (params (Velocity :type "Vector Structure"))
  (`/Engine/EditorBlueprintResources/StandardMacros.DoOnce` false
    (:`Completed`
      (`self.K2_DetachFromActor` "KeepWorld" "KeepWorld" "KeepWorld")
      (set `MovementComponent.Velocity` Velocity (`self.ProjectileMovement`))
      (`ActorComponent.SetActive` (`self.ProjectileMovement`) true false)
      (`KismetSystemLibrary.Delay` 0.3)
      (`PrimitiveComponent.SetCollisionEnabled` (`self.Grenade`) "QueryAndPhysics"))))

(fn `Explod`
  (`GameplayStatics.SpawnEmitterAtLocation` "/Game/StarterContent/Particles/P_Explosion.P_Explosion" (`SceneComponent.K2_GetComponentLocation` (`self.Grenade`)) (struct) (2.0 2.0 2.0))
  (`RadialForceComponent.FireImpulse` (`self.RadialForce`))
  (`GameplayStatics.PlaySoundAtLocation` (`self.ExplosionSound`) (`SceneComponent.K2_GetComponentLocation` (`self.Grenade`)) (struct) 0.5 1.0 0.0 null null null null)
  (`self.K2_DestroyActor`))

(fn `UserConstructionScript`)