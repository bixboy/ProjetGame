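; Base zombie enemy character that attacks players, tears planks off a barricaded window and vaults through it.
; Setup creates health and vaulting components and targets the first BP_WindowPlank found; damage feeds health and dismemberment, while death notifies BP_EnemyAI and ragdolls the mesh.
; Server/client event pairs drive plank pulling, using montage notifies and hand IK, and vault positioning via AI move with a timeline fallback, then rotation before vaulting.
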(event `self.ReceiveBeginPlay`
  (`self.SetupEnemy`))

(event `/Game/BP_/Interface/BPI_Health.TakeDamage`
  (params (Instigator :type "Actor Object Reference") (InstantKill :type Boolean) (Damage :type "Float (double-precision)") (ImpactPoint :type "Vector Structure") (HitBone :type Name))
  ;[0.06771 0.06771 0.06771] Health
  (`/Game/BP_/BP_Component/BPC_Health.TakeDamage` (`self.HealthComponent`) Instigator InstantKill false Damage ImpactPoint HitBone)
  (`self.Dismember` HitBone ImpactPoint))

(event `RagdollClient`
  (params (ImpulsePoint :type "Vector Structure") (BoneHit :type Name))
  ;[0.06771 0.06771 0.06771] Health
  (`self.StartRagdoll` ImpulsePoint BoneHit))

(event `/Game/BP_/Interface/BPI_Health.Death`
  (params (ImpulsePoint :type "Vector Structure") (BoneHit :type Name))
  ;[0.06771 0.06771 0.06771] Health
  (`self.StartDeath` ImpulsePoint BoneHit))

(event `self.AttackCollision.OnComponentBeginOverlap`
  (params (OverlappedComponent :type "PrimitiveComponent Object Reference") (OtherActor :type "Actor Object Reference") (OtherComp :type "PrimitiveComponent Object Reference") (OtherBodyIndex :type Integer) (bFromSweep :type Boolean) (SweepResult :type "HitResult Structure (by ref)"))
  ;[0.06771 0.06771 0.06771] Zombie Attack
  (if (`self.CanDamage`)
    (bind _asbp_player (cast `/Game/BP_/Game/Player/BP_Player` OtherActor))
    (`/Game/BP_/Game/Player/BP_Player.TakeDamage` _asbp_player false (`self.Damage`) (0.0 0.0 0.0) "None" null)))

(event `AttackAnimServer`
  ;[0.06771 0.06771 0.06771] Zombie Attack
  (`self.AttackAnim`))

(event `/Game/BP_/Interface/BPI_Enemy.CanAttack`
  (params (TrueFalse :type Boolean))
  ;[0.06771 0.06771 0.06771] Zombie Attack
  (set `self.CanDamage` TrueFalse))

(event `oui`
  (bind _plank (`/Game/BP_/Game/WorldProps/WindowPlank/BP_WindowPlank.GetPlank` (`self.WindowTarget`)))
  (`self.non` _plank))

(event `non`
  (params (CurrentPlank :type "StaticMeshComponent Object Reference"))
  (set `self.CurrentPlank` CurrentPlank))

(event `/Game/BP_/Interface/BPI_Enemy.RemovePlanke`
  (`self.removePlankServer`))

(event `RemovePlankClient`
  (bind (_returnvalue_roll _returnvalue_pitch _returnvalue_yaw) (`KismetMathLibrary.BreakRotator` (`KismetMathLibrary.FindLookAtRotation` (`SceneComponent.K2_GetComponentLocation` (`self.CapsuleComponent`)) (`SceneComponent.K2_GetComponentLocation` (`/Game/BP_/Game/WorldProps/WindowPlank/BP_WindowPlank.MiddlePoint` (`self.WindowTarget`))))))
  (set `/Game/BP_/Game/WorldProps/WindowPlank/BP_WindowPlank.CanRemovePlank` false (`self.WindowTarget`))
  (`self.oui`)
  (`SceneComponent.K2_SetWorldRotation` (`self.CapsuleComponent`) (`KismetMathLibrary.MakeRotator` 0.0 0.0 _returnvalue_yaw) false false)
  (`|PlayMontage` (`self.Mesh`) "/Game/Animations/ZombieAnim/AM_ZombiePullPlank.AM_ZombiePullPlank" 0.6
    (:`OnCompleted`
      (set `/Game/BP_/Game/WorldProps/WindowPlank/BP_WindowPlank.CanRemovePlank` true (`self.WindowTarget`))
      (`self.ToggleHandIK` false))
    (:`OnNotifyBegin`
      (if (not (`self.HavePlank`))
        (`self.ToggleHandIK` false)
        (`SceneComponent.K2_AttachToComponent` (`self.CurrentPlank`) (`self.Mesh`) "RightHand" "KeepWorld" "KeepWorld" "KeepWorld" true)
        (`KismetSystemLibrary.MoveComponentTo` (`self.CurrentPlank`) (0.0 0.0 0.0) (`SceneComponent.RelativeRotation` (`self.CurrentPlank`)))
        (set `self.HavePlank` true)
        (`/Game/BP_/Game/WorldProps/WindowPlank/BP_WindowPlank.RemovePlank` (`self.WindowTarget`) (`self.CurrentPlank`))
        (else
          (`SceneComponent.K2_DetachFromComponent` (`self.CurrentPlank`) "KeepWorld" "KeepWorld" "KeepWorld" true)
          (`PrimitiveComponent.SetSimulatePhysics` (`self.CurrentPlank`) true)
          (set `self.HavePlank` false))))))

(event `RemovePlankServer`
  (`self.RemovePlankClient`))

(event `/Game/BP_/Interface/BPI_Enemy.ToggleHandIK`
  (params (Enable :type Boolean) (Target :type "Vector Structure"))
  (message `/Game/BP_/Interface/BPI_Enemy.ToggleHandIK` (`SkeletalMeshComponent.GetAnimInstance` (`self.Mesh`)) Enable (`SceneComponent.K2_GetComponentLocation` (`self.CurrentPlank`))))

(event `/Game/BP_/Interface/BPI_Enemy.MoveToVoltingPose`
  (`self.Server`))

(event `Client`
  (bind (_returnvalue_location _returnvalue_rotation) (`KismetMathLibrary.BreakTransform` (`SceneComponent.K2_GetComponentToWorld` (`self.CapsuleComponent`))))
  (bind (_returnvalue_location_2 _returnvalue_rotation_2) (`KismetMathLibrary.BreakTransform` (`SceneComponent.K2_GetComponentToWorld` (`/Game/BP_/Game/WorldProps/WindowPlank/BP_WindowPlank.InsidePoint` (`self.WindowTarget`)))))
  ;[0.08854 0.08854 0.08854] Vaulting
  (`|AIMoveTo` self (`SceneComponent.K2_GetComponentLocation` (`/Game/BP_/Game/WorldProps/WindowPlank/BP_WindowPlank.InsidePoint` (`self.WindowTarget`))) null
    (:`OnSuccess`
      (`/Engine/EditorBlueprintResources/StandardMacros.DoOnce` false :!label _label
        (:`Completed`
          (`self.RotateToWindow`))))
    (:`OnFail`
      (set `self.VaultStartTransform` (`KismetMathLibrary.MakeTransform` _returnvalue_location _returnvalue_rotation (`SceneComponent.K2_GetComponentScale` (`self.Mesh`))))
      (bind (_direction _alpha) (`Timeline|ForceMoveTL` :!via `PlayFromStart`)
        (:`Update`
          (`SceneComponent.K2_SetWorldTransform` (`self.CapsuleComponent`) (`KismetMathLibrary.TLerp` (`self.VaultStartTransform`) (`KismetMathLibrary.MakeTransform` _returnvalue_location_2 _returnvalue_rotation_2) _alpha) false false))
        (:`Finished`
          (goto _label))))))

(event `Server`
  (`self.Client`))

(event `CustomEvent`
  ;[0.08854 0.08854 0.08854] Vaulting
  (`/Game/BP_/BP_Component/BPC_Vaulting.ResetVault` (`self.BPC_Vaulting`))
  (set `self.OnMap` true))

(event `RotateToWindow`
  ;[0.08854 0.08854 0.08854] Vaulting
  (set `self.RotateStart` (`SceneComponent.K2_GetComponentRotation` (`self.CapsuleComponent`)))
  (bind (_direction _alpha) (`Timeline|RotateToWindowTL` :!via `PlayFromStart`)
    (:`Update`
      (`SceneComponent.K2_SetWorldRotation` (`self.CapsuleComponent`) (`KismetMathLibrary.RLerp` (`self.RotateStart`) (`SceneComponent.K2_GetComponentRotation` (`/Game/BP_/Game/WorldProps/WindowPlank/BP_WindowPlank.MiddlePoint` (`self.WindowTarget`))) _alpha) false false))
    (:`Finished`
      (`/Game/BP_/BP_Component/BPC_Vaulting.GetInitialObjectLocation` (`self.BPC_Vaulting`)))))

(event `/Game/BP_/Interface/BPI_Vaulting.ResetVault`
  ;[0.08854 0.08854 0.08854] Vaulting
  (`/Game/BP_/BP_Component/BPC_Vaulting.ResetVault` (`self.BPC_Vaulting`))
  (set `self.OnMap` true))

(fn `Attack`
  (returns (AnimLength :type "Float (double-precision)"))
  (`self.AttackAnimServer`)
  (return (`self.AttackLength`)))

(fn `AttackAnim`
  (bind _returnvalue (`self.PlayAnimMontage` (`self.AnimAttack`)))
  (set `self.AttackLength` _returnvalue)
  (return))

(fn `Dismember`
  (params (HitBone :type Name) (ImpactPoint :type "Vector Structure"))
  (`/Game/BP_/BP_Component/BPC_Dismembrement.renameBones` (`self.BPC_Dismembrement`) HitBone ImpactPoint))

(fn `GetOnMap`
  (returns (OnMap :type Boolean))
  (return (`self.OnMap`)))

(fn `GetWindowLocation`
  (returns (Window :type "/Game/BP_/Game/WorldProps/WindowPlank/BP_WindowPlank Object Reference"))
  (return (`self.WindowTarget`)))

(fn `SetupEnemy`
  (bind _returnvalue (`AddComponent|NODE_AddBPC_Health-0` :`MaxHealth` (`self.Health`)))
  (set `self.HealthComponent` _returnvalue)
  (bind _returnvalue_2 (`GameplayStatics.GetActorOfClass` "/Game/BP_/Game/WorldProps/WindowPlank/BP_WindowPlank.BP_WindowPlank_C"))
  (set `self.WindowTarget` _returnvalue_2)
  (bind _returnvalue_3 (`|AddComponentByClass` "/Game/BP_/BP_Component/BPC_Vaulting.BPC_Vaulting_C" (`self.MotionWarping`) "/Game/Animations/ZombieAnim/AM_ZombieVaultOver.AM_ZombieVaultOver" (`self.CharacterMovement`) (`self.CapsuleComponent`) (`self.Mesh`)))
  (set `self.BPC_Vaulting` _returnvalue_3))

(fn `StartDeath`
  (params (ImpulsePoint :type "Vector Structure") (BoneHit :type Name))
  (bind _asbp_enemy_ai (cast `/Game/BP_/Game/Enemy/BP_EnemyAI` (`AIBlueprintHelperLibrary.GetAIController` self)))
  (`/Game/BP_/Game/Enemy/BP_EnemyAI.Death` _asbp_enemy_ai)
  (`self.RagdollClient` (`local.ImpulsePoint`) (`local.BoneHit`)))

(fn `StartRagdoll`
  (params (ImpulsePoint :type "Vector Structure") (BoneHit :type Name))
  (bind _mesh (`self.Mesh`))
  (`|ExecutionSequence`
    (:`then_0`
      (`CharacterMovementComponent.DisableMovement` (`self.CharacterMovement`))
      (`SkeletalMeshComponent.Stop` (`self.Mesh`)))
    (:`then_1`
      (`PrimitiveComponent.SetCollisionEnabled` (`self.CapsuleComponent`) "NoCollision")
      (`CharacterMovementComponent.SetMovementMode` (`self.CharacterMovement`) "MOVE_None" 0)
      (`PrimitiveComponent.SetCollisionObjectType` _mesh "ECC_PhysicsBody")
      (`PrimitiveComponent.SetCollisionEnabled` _mesh "QueryAndPhysics")
      (`SkeletalMeshComponent.SetAllBodiesBelowSimulatePhysics` (`self.Mesh`) "Hips" true true)
      (`PrimitiveComponent.AddImpulse` (`self.Mesh`) (* (`local.ImpulsePoint`) 10.0) (`local.BoneHit`) false))))

(fn `UserConstructionScript`)