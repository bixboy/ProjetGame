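; BP_PlayerLobby is the player representation in the lobby, showing that player's lobby info on a widget component.
; UpdateLobbyInfo sets the PlayerLobbyInfo variable, whose RepNotify passes it to the WB_PlayerLobbyInfo widget and makes the component visible.
; If the widget is not yet valid, the RepNotify retries itself on a short timer until it is.
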(fn `OnRep_PlayerLobbyInfo`
  (bind _returnvalue (`WidgetComponent.GetWidget` (`self.Lobbyinfo`)))
  (`/Engine/EditorBlueprintResources/StandardMacros.IsValid` _returnvalue
    (:`Is Valid`
      (bind _aswb_player_lobby_info (cast `/Game/BP_/Lobby/Widgets/WB_PlayerLobbyInfo` _returnvalue))
      (`/Game/BP_/Lobby/Widgets/WB_PlayerLobbyInfo.Update` _aswb_player_lobby_info (`self.PlayerLobbyInfo`))
      (`SceneComponent.SetVisibility` (`self.Lobbyinfo`) true false))
    (:`Is Not Valid`
      (`KismetSystemLibrary.K2_SetTimer` null "OnRep_PlayerLobbyInfo" 0.1))))

(fn `UpdateLobbyInfo`
  (params (PlayerLobbyInfo :type "/Game/BP_/Lobby/S_PlayerLobbyInfo Structure"))
  (set `self.PlayerLobbyInfo` PlayerLobbyInfo))

(fn `UserConstructionScript`)