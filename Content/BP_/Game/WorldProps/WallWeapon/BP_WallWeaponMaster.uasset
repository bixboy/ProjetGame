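; BP_WallWeaponMaster is the base wall-buy weapon prop, selling a weapon to a player who interacts with it.
; Interact calls BuyWeaponClient, which compares the player's BPCScore score to Price and adds the Weapon class to the player as a component.
; Only for the locally controlled player does it subtract the price through SubstractServer and play the payment sound at the prop's location.
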(event `self.ReceiveBeginPlay`)

(event `/Game/BP_/Interface/BPI_Interaction.Interact`
  (params (Player :type "/Game/BP_/Game/Player/BP_Player Object Reference"))
  (`self.BuyWeaponClient` Player))

(event `BuyWeaponClient`
  (params (Player :type "/Game/BP_/Game/Player/BP_Player Object Reference"))
  (if (>= (`/Game/BP_/BP_Component/BPC_Score.Score` (`/Game/BP_/Game/Player/BP_Player.BPC_Score` Player)) (`self.Price`))
    (`|AddComponentByClass` :`self` Player :`Class` (`self.Weapon`))
    (if (`Pawn.IsLocallyControlled` Player)
      (`/Game/BP_/BP_Component/BPC_Score.SubstractServer` (`/Game/BP_/Game/Player/BP_Player.BPC_Score` Player) (`self.Price`))
      (`GameplayStatics.PlaySoundAtLocation` "/Game/SFX/Sounds/Kaching_Pay.Kaching_Pay" (`self.K2_GetActorLocation`) (struct) 1.0 1.0 0.0 null null null null))))

(fn `UserConstructionScript`
  (`parent.UserConstructionScript`))