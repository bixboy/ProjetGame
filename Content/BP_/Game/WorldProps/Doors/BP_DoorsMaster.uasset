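; Master door Blueprint that the player opens by paying a price from their score.
; Interact stores the player and calls OpenDoor, which checks the player's BPC Score component against Price and deducts it through SubstractServer when affordable.
; OpenEffect then sets IsOpen and destroys the door rather than animating it, with the IsOpen RepNotify also destroying the actor.
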(event `/Game/BP_/Interface/BPI_Interaction.Interact`
  (params (Player :type "/Game/BP_/Game/Player/BP_Player Object Reference"))
  (bind _output_get (set `self.Player` Player))
  (`self.Open Door` _output_get))

(event `OpenEffect`
  (set `self.IsOpen` true)
  (`self.K2_DestroyActor`))

(fn `OnRep_IsOpen`
  (`self.K2_DestroyActor`))

(fn `Open Door`
  (params (Player :type "/Game/BP_/Game/Player/BP_Player Object Reference"))
  (if (>= (`/Game/BP_/BP_Component/BPC_Score.Score` (`/Game/BP_/Game/Player/BP_Player.BPC_Score` Player)) (`self.Price`))
    (`/Game/BP_/BP_Component/BPC_Score.SubstractServer` (`/Game/BP_/Game/Player/BP_Player.BPC_Score` Player) (`self.Price`))
    (`self.OpenEffect`)))

(fn `UserConstructionScript`
  (`parent.UserConstructionScript`))