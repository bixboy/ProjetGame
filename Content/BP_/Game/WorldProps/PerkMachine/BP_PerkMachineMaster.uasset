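; Base perk machine world prop that sells its current perk to an interacting player for score once powered.
; Interact calls TakePerkClient, which checks the player's score against the price and the power state, then adds the perk.
; Only the locally controlled player requests the score deduction through the score component's SubstractServer.
; SetPowerOn enables purchases and the logo's roll spin, advanced a fixed step each Tick regardless of frame time.
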(event `/Game/BP_/Interface/BPI_Interaction.Interact`
  (params (Player :type "/Game/BP_/Game/Player/BP_Player Object Reference"))
  (`self.TakePerkClient` Player))

(event `TakePerkClient`
  (params (Player :type "/Game/BP_/Game/Player/BP_Player Object Reference"))
  (if (and (>= (`/Game/BP_/BP_Component/BPC_Score.Score` (`/Game/BP_/Game/Player/BP_Player.BPC_Score` Player)) (`self.Price`)) (`self.PowerOn`))
    (`/Game/BP_/Game/Player/BP_Player.AddPerk` Player (`self.CurrentPerk`))
    (if (`Pawn.IsLocallyControlled` Player)
      (`/Game/BP_/BP_Component/BPC_Score.SubstractServer` (`/Game/BP_/Game/Player/BP_Player.BPC_Score` Player) (`self.Price`)))))

(event `self.ReceiveTick`
  (params (DeltaSeconds :type "Float (single-precision)"))
  (bind (_relativerotation_roll _relativerotation_pitch _relativerotation_yaw) (`KismetMathLibrary.BreakRotator` (`SceneComponent.RelativeRotation` (`self.PerkLogo`))))
  (if (`self.PowerOn`)
    (`SceneComponent.K2_SetRelativeRotation` (`self.PerkLogo`) (`KismetMathLibrary.MakeRotator` (+ _relativerotation_roll 0.5) _relativerotation_pitch _relativerotation_yaw) false false)))

(event `SetPowerOn`
  (set `self.PowerOn` true))

(fn `UserConstructionScript`
  (`parent.UserConstructionScript`))