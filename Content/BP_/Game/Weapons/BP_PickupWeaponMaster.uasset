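; BP_PickupWeaponMaster is a weapon pickup, named as the master for such pickups, that grants a weapon to the player.
; When its sphere collision is overlapped by an actor whose class is exactly BP_Player, it adds a WeaponToSpawn component to that player and destroys itself.
; GetWeaponClass returns a separate WeaponClass variable, while GetWeapon and the construction script are empty.
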(event `self.SphereCollision.OnComponentBeginOverlap`
  (params (OverlappedComponent :type "PrimitiveComponent Object Reference") (OtherActor :type "Actor Object Reference") (OtherComp :type "PrimitiveComponent Object Reference") (OtherBodyIndex :type Integer) (bFromSweep :type Boolean) (SweepResult :type "HitResult Structure (by ref)"))
  (if (== (`GameplayStatics.GetObjectClass` OtherActor) "/Game/BP_/Game/Player/BP_Player.BP_Player_C")
    (bind _asbp_player (cast `/Game/BP_/Game/Player/BP_Player` OtherActor))
    (`|AddComponentByClass` :`self` _asbp_player :`Class` (`self.WeaponToSpawn`))
    (`self.K2_DestroyActor`)))

(fn `GetWeapon`
  (returns (Weapon :type "/Game/BP_/Game/Weapons/BPC_WeaponMaser Object Reference"))
  (return null))

(fn `GetWeaponClass`
  (returns (WeaponClass :type "/Game/BP_/Game/Weapons/Enum/Enum_WeaponClass Enum"))
  (return (`self.WeaponClass`)))

(fn `UserConstructionScript`)