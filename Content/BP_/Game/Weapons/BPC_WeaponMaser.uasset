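; BPC_WeaponMaser is a player weapon component that registers as primary or secondary and attaches to first- or third-person mesh sockets.
; Input cycles single, burst-style semi-auto (timer plus DoN) and looping full-auto fire, consuming ammo with animation and camera shake.
; On the server, a camera trace feeds a barrel trace with random spread, tighter when aiming, then spawns projectiles and ejected casings.
; Reload plays interruptible animations without refilling ammo.
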(event `self.ReceiveBeginPlay`
  (bind _asbp_player (cast `/Game/BP_/Game/Player/BP_Player` (`self.GetOwner`)))
  (set `self.Player` _asbp_player)
  (`self.PickupWeapon`)
  (`self.UpdateAmmo` true)
  (`self.AttachWeapon` "GripWeapon" "GripPoint")
  (message `/Game/BP_/Interface/BPI_Weapon.SetAim` (`self.GetAnimInstance` (`/Game/BP_/Game/Player/BP_Player.FirstPersonMesh` (`self.Player`)))))

(event `EnhancedInput|/Game/BP_/Inputs/Actions/Weapon/IA_FireMode`
  (params (ActionValue :type Boolean) (ElapsedSeconds :type "Float (double-precision)") (TriggeredSeconds :type "Float (double-precision)") (InputAction :type "InputAction Object Reference" :default "/Game/BP_/Inputs/Actions/Weapon/IA_FireMode.IA_FireMode"))
  (:`Started`
    (if (`self.CanChangeFireMode`)
      (bind _output_get (set `self.FireMode` (select `/Game/BP_/Game/Weapons/Enum/Enum_FireMode` (`self.FireMode`) :`NewEnumerator2` "NewEnumerator1" :`NewEnumerator1` "NewEnumerator0" :`NewEnumerator0` "NewEnumerator2" :!type "/Game/BP_/Game/Weapons/Enum/Enum_FireMode Enum")))
      (`KismetSystemLibrary.PrintString` (`|GetEnumeratorNameAsString` _output_get)))))

(event `EnhancedInput|/Game/BP_/Inputs/Actions/Weapon/IA_Reaload`
  (params (ActionValue :type Boolean) (ElapsedSeconds :type "Float (double-precision)") (TriggeredSeconds :type "Float (double-precision)") (InputAction :type "InputAction Object Reference" :default "/Game/BP_/Inputs/Actions/Weapon/IA_Reaload.IA_Reaload"))
  (:`Started`
    (`self.Reaload` :!label _label)))

(event `/Game/BP_/Interface/BPI_Weapon.Fire`
  (params (Cancel :type Boolean))
  ;[0.06301 0.06301 0.06301] Fire/Shoot
  (if (not Cancel)
    (`self.StartFire` :!label _label_2)
    (else
      (goto _label_2 :!via `execute2`))))

(event `StopReaload`
  (goto _label :!via `StopRealoading`))

(event `StartSemiAuto`
  ;[0.0625 0.0625 0.0625] Semi Auto Shoot
  (bind _returnvalue (`KismetSystemLibrary.K2_SetTimerDelegate` (delegate `SemiAutoFire`) 0.1 true (* 0.1 -1.0)))
  (set `self.SemiAutoHandel` _returnvalue))

(event `SemiAutoFire`
  ;[0.0625 0.0625 0.0625] Semi Auto Shoot
  (bind _counter (`/Engine/EditorBlueprintResources/StandardMacros.Do N` (`self.SemiAutoShot`) :!label _label_3)
    (:`Exit`
      (if (> (`self.CurrentAmmo`) 0)
        (`|ExecutionSequence`
          (:`then_0`
            (`self.Aiming`)
            (`self.UpdateAmmo` false true)
            (`self.PlayAnimation` (`self.FireWeaponSK`))
            (`self.Shake`))
          (:`then_1`
            (if (== _counter (`self.SemiAutoShot`))
              (`KismetSystemLibrary.K2_ClearAndInvalidateTimerHandle` (`self.SemiAutoHandel`))
              (`KismetSystemLibrary.Delay` 0.2)
              (set `self.CanFire` true)
              (goto _label_3 :!via `Reset`))))))))

(event `ResetSemiAuto`
  ;[0.0625 0.0625 0.0625] Semi Auto Shoot
  (`KismetSystemLibrary.K2_ClearAndInvalidateTimerHandle` (`self.SemiAutoHandel`))
  (goto _label_3 :!via `Reset`))

(event `SpawnBullet`
  (params (StartLocation :type "Vector Structure") (TargetLocation :type "Vector Structure"))
  (`self.SpawnBullets` StartLocation TargetLocation))

(event `RealoadWeapon`
  (params (PlayerMeshTP :type "SkeletalMeshComponent Object Reference") (PlayerMeshFP :type "SkeletalMeshComponent Object Reference"))
  (`|PlayMontage` PlayerMeshFP (`self.AnimRealoadFP`)
    (:`then`
      (`|PlayMontage` PlayerMeshTP (`self.AnimRealoadTP`)
        (:`then`
          (`self.PlayAnimation` self (`self.AnimReload`) false))))))

(fn `Aiming`
  (locals (FirstLineTraceFire :type "Vector Structure") (TargetLocation :type "Vector Structure") (BoneHite :type Name))
  (bind _returnvalue (`self.GetSocketLocation` "barrel"))
  (bind _returnvalue_2 (`self.GetSocketLocation` "barrel"))
  (bind _returnvalue_3 (- (`local.FirstLineTraceFire`) _returnvalue_2))
  (bind _returnvalue_4 (- (`local.FirstLineTraceFire`) _returnvalue))
  (bind _firstpersoncamera (`/Game/BP_/Game/Player/BP_Player.FirstPersonCamera` (`self.Player`)))
  (bind _returnvalue_5 (`self.K2_GetComponentLocation` _firstpersoncamera))
  (if (`KismetSystemLibrary.IsServer`)
    (bind _outhit (`KismetSystemLibrary.LineTraceSingle` :`Start` _returnvalue_5 :`End` (+ _returnvalue_5 (* (`KismetMathLibrary.GetForwardVector` (`self.K2_GetComponentRotation` _firstpersoncamera)) (`self.Range`))) :`TraceChannel` "TraceTypeQuery4" :`TraceColor` (struct :`R` 0.070212 :`B` 1.0 :`A` 1.0)))
    (bind (_bblockinghit _binitialoverlap _time _distance _location _impactpoint _normal _impactnormal _physmat _hitactor _hitcomponent _hitbonename _bonename _hititem _elementindex _faceindex _tracestart _traceend) (`GameplayStatics.BreakHitResult` _outhit))
    (if (`KismetSystemLibrary.DoesImplementInterface` _hitactor)
      (set `local.FirstLineTraceFire` _impactpoint)
      (else
        (set `local.FirstLineTraceFire` _traceend)))
    (if (`self.hasAiming`)
      (bind _outhit_2 (`KismetSystemLibrary.LineTraceSingle` :`Start` _returnvalue_2 :`End` (+ (* (/ _returnvalue_3 (`KismetMathLibrary.VSize` _returnvalue_3)) 15000.0) (`local.FirstLineTraceFire`) (`KismetMathLibrary.MakeVector` (`KismetMathLibrary.RandomFloatInRange` -250.0 250.0) (`KismetMathLibrary.RandomFloatInRange` -250.0 250.0) (`KismetMathLibrary.RandomFloatInRange` -250.0 250.0))) :`TraceChannel` "TraceTypeQuery5" :`TraceColor` (struct :`R` 0.064483 :`B` 1.0 :`A` 1.0)))
      (bind (_bblockinghit_2 _binitialoverlap_2 _time_2 _distance_2 _location_2 _impactpoint_2 _normal_2 _impactnormal_2 _physmat_2 _hitactor_2 _hitcomponent_2 _hitbonename_2 _bonename_2 _hititem_2 _elementindex_2 _faceindex_2 _tracestart_2 _traceend_2) (`GameplayStatics.BreakHitResult` _outhit_2))
      (if (`KismetSystemLibrary.DoesImplementInterface` _hitactor_2 "/Game/BP_/Interface/BPI_Health.BPI_Health_C")
        (set `local.BoneHite` _hitbonename_2)
        (set `local.TargetLocation` _impactpoint_2)
        (else
          (set `local.TargetLocation` _traceend_2)))
      (`self.SpawnBullet` _tracestart_2 (`local.TargetLocation`))
      (else
        (bind _outhit_3 (`KismetSystemLibrary.LineTraceSingle` _returnvalue (+ (* (/ _returnvalue_4 (`KismetMathLibrary.VSize` _returnvalue_4)) 15000.0) (`local.FirstLineTraceFire`) (`KismetMathLibrary.MakeVector` (`KismetMathLibrary.RandomFloatInRange` -750.0 750.0) (`KismetMathLibrary.RandomFloatInRange` -750.0 750.0) (`KismetMathLibrary.RandomFloatInRange` -750.0 750.0))) "TraceTypeQuery5"))
        (bind (_bblockinghit_3 _binitialoverlap_3 _time_3 _distance_3 _location_3 _impactpoint_3 _normal_3 _impactnormal_3 _physmat_3 _hitactor_3 _hitcomponent_3 _hitbonename_3 _bonename_3 _hititem_3 _elementindex_3 _faceindex_3 _tracestart_3 _traceend_3) (`GameplayStatics.BreakHitResult` _outhit_3))
        (if (`KismetSystemLibrary.DoesImplementInterface` _hitactor_3 "/Game/BP_/Interface/BPI_Health.BPI_Health_C")
          (set `local.BoneHite` _hitbonename_3)
          (set `local.TargetLocation` _impactpoint_3)
          (else
            (set `local.TargetLocation` _traceend_3)))
        (`self.SpawnBullet` _tracestart_3 (`local.TargetLocation`))))))

(fn `AttachWeapon`
  (params (SocketNameTP :type Name) (SocketNameFP :type Name))
  (bind _player (`self.Player`))
  (set `/Game/BP_/Game/Player/BP_Player.CurrentWeapon` self _player)
  (if (`Pawn.IsLocallyControlled` (`self.Player`))
    (`self.K2_AttachToComponent` (`/Game/BP_/Game/Player/BP_Player.FirstPersonMesh` _player) (`local.SocketNameFP`) "KeepRelative" "KeepRelative" "KeepRelative")
    (else
      (`self.K2_AttachToComponent` (`/Game/BP_/Game/Player/BP_Player.TP_Body` (`self.Player`)) (`local.SocketNameTP`) "KeepRelative" "KeepRelative" "KeepRelative"))))

(fn `EquipWeapon`
  (`self.ResetSemiAuto`)
  (`self.AttachWeapon` "GripWeapon" "GripPoint"))

(fn `GetWeapon`
  (returns (Weapon :type "/Game/BP_/Game/Weapons/BPC_WeaponMaser Object Reference"))
  (return self))

(fn `GetWeaponClass`
  (returns (WeaponClass :type "/Game/BP_/Game/Weapons/Enum/Enum_WeaponClass Enum"))
  (return "NewEnumerator0"))

(fn `PickupWeapon`
  (bind _player (`self.Player`))
  (switch `/Game/BP_/Game/Weapons/Enum/Enum_WeaponClass` (`self.WeaponClass`)
    (:`NewEnumerator0`
      (bind _primaryweapon (`/Game/BP_/Game/Player/BP_Player.PrimaryWeapon` (`self.Player`))
        (:`then`
          (`self.K2_DestroyComponent` _primaryweapon))
        (:`else`
          _))
      (set `/Game/BP_/Game/Player/BP_Player.PrimaryWeapon` self (`self.Player`))
      (set `/Game/BP_/Game/Player/BP_Player.HasPrimaryWeapon` true (`self.Player`))
      (bind _secondaryweapon (`/Game/BP_/Game/Player/BP_Player.SecondaryWeapon` (`self.Player`))
        (:`then`
          (`self.UnequipWeapon` _secondaryweapon "GripSideWeapon"))
        (:`else`
          _)))
    (:`NewEnumerator1`
      (bind _secondaryweapon_2 (`/Game/BP_/Game/Player/BP_Player.SecondaryWeapon` (`self.Player`))
        (:`then`
          (`self.K2_DestroyComponent` _secondaryweapon_2))
        (:`else`
          _))
      (set `/Game/BP_/Game/Player/BP_Player.SecondaryWeapon` self (`self.Player`))
      (set `/Game/BP_/Game/Player/BP_Player.HasSecondaryWeapon` true (`self.Player`))
      (bind _primaryweapon_2 (`/Game/BP_/Game/Player/BP_Player.PrimaryWeapon` (`self.Player`))
        (:`then`
          (`self.UnequipWeapon` _primaryweapon_2 "GripBackWeapon"))
        (:`else`
          _))))
  (set `/Game/BP_/Game/Player/BP_Player.CurrentWeaponINT` (`KismetMathLibrary.Conv_ByteToInt` (`self.WeaponName`)) _player)
  (set `/Game/BP_/Game/Player/BP_Player.CurrentWeapon` self _player))

(fn `Shake`
  (if (`Pawn.IsLocallyControlled` (`self.Player`))
    (`PlayerController.ClientStartCameraShake` :`self` (`/Game/BP_/Game/Player/BP_Player.getPlayerController` (`self.Player`)) :`Shake` "/Game/BP_/Game/Weapons/Shake/BP_ShakeFire.BP_ShakeFire_C" :`PlaySpace` "UserDefined")))

(fn `SpawnAmmoCasing`
  (bind _returnvalue (`self.GetSocketRotation` "AmmoEject"))
  (bind _returnvalue_2 (`|SpawnActorFromClass` (`self.AmmoEjection`) (`KismetMathLibrary.MakeTransform` (`self.GetSocketLocation` "AmmoEject") (`KismetMathLibrary.MakeRotator` (.roll _returnvalue) (- (.pitch _returnvalue) 90.0) (.yaw _returnvalue))) "Undefined" "MultiplyWithRoot" null null))
  (bind _ammo (`/Game/BP_/Game/Weapons/projectiles/AmmoEjected/Bp_AmmoEjectedMaster.Ammo` _returnvalue_2))
  (`self.AddImpulse` _ammo (+ (* (`KismetMathLibrary.GetRightVector` _returnvalue) (`KismetMathLibrary.RandomFloatInRange` 90.0 150.0)) (* (`KismetMathLibrary.GetForwardVector` _returnvalue) (`KismetMathLibrary.RandomFloatInRange` 20.0 20.0))) "None" true)
  (`self.AddAngularImpulseInRadians` _ammo (`KismetMathLibrary.MakeVector` 0.0 50.0 (`KismetMathLibrary.RandomFloatInRange` -100.0 150.0)) "None" true))

(fn `SpawnBullets`
  (params (Start :type "Vector Structure (by ref)") (Target :type "Vector Structure (by ref)"))
  (bind _player (`self.Player`))
  (`|SpawnActorFromClass` "/Game/BP_/Game/Weapons/projectiles/BP_ProjectileMaster.BP_ProjectileMaster_C" (`KismetMathLibrary.MakeTransform` (`self.GetSocketLocation` "barrel") (`KismetMathLibrary.FindLookAtRotation` Start Target)) "Undefined" "MultiplyWithRoot" _player (`self.Damage`) "/Engine/EditorMeshes/ArcadeEditorSphere.ArcadeEditorSphere" _player)
  (`self.SpawnAmmoCasing`))

(fn `UnequipWeapon`
  (params (SocketName :type Name))
  (`self.K2_AttachToComponent` (`/Game/BP_/Game/Player/BP_Player.TP_Body` (`self.Player`)) SocketName "KeepRelative" "KeepRelative" "KeepRelative")
  (`self.ResetSemiAuto`)
  (`self.StopReaload`))

(fn `UpdateAmmo`
  (params (FullAmmo :type Boolean) (Substract :type Boolean))
  (if FullAmmo
    (set `self.CurrentAmmo` (`self.MaxAmmo`))
    (elif Substract
      (bind _result (`/Engine/EditorBlueprintResources/StandardMacros.DecrementInt` (`self.CurrentAmmo`))
        (:`  `
          (set `self.CurrentAmmo` (`KismetMathLibrary.Clamp` _result 0 (`self.MaxAmmo`))))))))