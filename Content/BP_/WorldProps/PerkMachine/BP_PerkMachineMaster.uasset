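; BP_PerkMachineMaster is a base perk machine world prop that grants its configured perk to a player who interacts with it.
; A PowerOn flag, set by the SetPowerOn event, gates both the interaction and the logo animation.
; While powered, Tick spins the PerkLogo component by adding a fixed roll step each frame, so the spin speed depends on frame rate.
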(event `/Game/BP_/Interface/BPI_Interaction.Interact`
  (params (Player :type "/Game/BP_/Player/BP_Player Object Reference"))
  (if (`self.PowerOn`)
    (`/Game/BP_/Player/BP_Player.AddPerk` Player (`self.CurrentPerk`))))

(event `self.ReceiveTick`
  (params (DeltaSeconds :type "Float (single-precision)"))
  (bind (_relativerotation_roll _relativerotation_pitch _relativerotation_yaw) (`KismetMathLibrary.BreakRotator` (`SceneComponent.RelativeRotation` (`self.PerkLogo`))))
  (if (`self.PowerOn`)
    (`SceneComponent.K2_SetRelativeRotation` (`self.PerkLogo`) (`KismetMathLibrary.MakeRotator` (+ _relativerotation_roll 0.5) _relativerotation_pitch _relativerotation_yaw) false false)))

(event `SetPowerOn`
  (set `self.PowerOn` true))

(fn `UserConstructionScript`
  (`parent.UserConstructionScript`))