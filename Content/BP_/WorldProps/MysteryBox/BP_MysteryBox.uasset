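; Mystery box world prop that sells a random weapon for score points.
; Buying loads DT_Weapons, opens the lid and cycles random weapon meshes with growing delays as the rising display slows.
; A weighted roll on ChanceToSpawn picks the winner, which slowly sinks while available to take.
; Taking it adds its weapon component to the player; taking or timeout reverses the open timeline, resetting the box to Buy.
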(event `self.ReceiveBeginPlay`
  (`TimelineComponent.SetPlayRate` (`self.Open_TL`) (/ 1.0 (`self.OpeningSpeed`)))
  (`TimelineComponent.SetPlayRate` (`self.CloseTL`) (/ 1.0 (`self.ClosingSpeed`))))

(event `/Game/BP_/Interface/BPI_Interaction.Interact`
  (params (Player :type "/Game/BP_/Player/BP_Player Object Reference"))
  ;[0.06771 0.06771 0.06771] Interaction
  (set `self.Player` Player)
  (switch `/Game/BP_/WorldProps/MysteryBox/Enum_MysteryBox` (`self.State`)
    (:`NewEnumerator0`
      (`self.BuyBox` (`self.Player`)))
    (:`NewEnumerator1`
      (`self.TakeWeaponClient` (`self.Player`)))))

(event `TakeWeaponClient`
  (params (Player :type "/Game/BP_/Player/BP_Player Object Reference"))
  ;[0.06771 0.06771 0.06771] Interaction
  (`self.TakeWeapon` Player))

(event `OpenCrate`
  ;[0.06771 0.06771 0.06771] Open and close
  (`self.SpinBox`)
  (bind (_direction _alpha) (`Timeline|Open_TL` :!via `PlayFromStart` :!label _label)
    (:`Update`
      (`SceneComponent.K2_SetRelativeRotation` (`self.Top_Scene`) (`KismetMathLibrary.RLerp` (struct) (struct :`Roll` -150.0) _alpha) false false)
      (`SceneComponent.K2_SetRelativeLocation` (`self.Weapon`) (`KismetMathLibrary.VLerp` (`KismetMathLibrary.MakeVector` (`self.WeaponXLoc`)) (select `ETimelineDirection` _direction :`Forward` (`KismetMathLibrary.MakeVector` (`self.WeaponXLoc`) 0.0 90.0) :`Backward` (`self.WeaponLoc`)) _alpha) false false))
    (:`Finished`
      (switch `ETimelineDirection` _direction
        (:`Backward`
          (`self.SetState`))))))

(event `CloseBox`
  (bind (_relativelocation_x _relativelocation_y _relativelocation_z) (`KismetMathLibrary.BreakVector` (`SceneComponent.RelativeLocation` (`self.Weapon`))))
  ;[0.06771 0.06771 0.06771] Open and close
  (set `self.WeaponLoc` (`KismetMathLibrary.MakeVector` (`self.WeaponXLoc`) _relativelocation_y _relativelocation_z))
  (goto _label :!via `ReverseFromEnd`))

(event `CloseBoxSlowly`
  (bind (_direction _alpha) (`Timeline|CloseTL` :!via `PlayFromStart`)
    (:`Update`
      (`SceneComponent.K2_SetRelativeLocation` (`self.Weapon`) (`KismetMathLibrary.VLerp` (`KismetMathLibrary.MakeVector` (`self.WeaponXLoc`) 0.0 90.0) (`KismetMathLibrary.MakeVector` (`self.WeaponXLoc`) 0.0 60.0) _alpha) false false))
    (:`Finished`
      (if (`|EnumEquality` (`self.State`) "NewEnumerator1")
        (set `self.CanInteract` false)
        (`self.CloseBox`)))))

(event `SetWinerClient`
  (params (Weapon :type "/Game/BP_/Weapons/Enum/Struct_Weapon Structure"))
  (`self.SetWiner` Weapon))

(event `SpinBox`
  (if (< (`self.SpinIndex`) 50)
    (`self.SpinWeapon`)
    (else
      (`self.GetWinerServer`)
      (`self.SetWinerClient` (`self.WinnerWeapon`)))))

(event `GetWinerServer`
  (`self.GetWinerWeapon`))

(event `SetWinerWeaponClient`
  (params (Weapon :type "/Game/BP_/Weapons/Enum/Struct_Weapon Structure"))
  (set `self.WinnerWeapon` Weapon))

(event `SpinWeapon`
  (set `self.SpinIndexShow` (`KismetMathLibrary.RandomIntegerInRange` 1 (`self.RowAmount`)))
  (if (!= (`self.SpinIndexShow`) (`self.LastWeaponIndex`))
    (`KismetSystemLibrary.Delay` (/ (`KismetMathLibrary.FClamp` (- (`self.SpinIndex`) 20) 1.0 50.0) 100.0))
    (bind _returnvalue (`|GetDataTableRow` "/Game/BP_/Weapons/Enum/DT_Weapons.DT_Weapons" (`KismetStringLibrary.Conv_StringToName` (`KismetStringLibrary.Conv_IntToString` (`self.SpinIndexShow`))))
      (:`then`
        (`self.SetSkeletalMesh` (`.WeaponSK_18_82D305814B0EFC10FACFBDB9B552FD95` (break `/Game/BP_/Weapons/Enum/Struct_Weapon` _returnvalue)))
        (set `self.LastWeaponIndex` (`self.SpinIndexShow`))
        (`/Engine/EditorBlueprintResources/StandardMacros.IncrementInt` (`self.SpinIndex`)
          (:`  `
            (`self.SpinBox`)))))
    (else
      (`self.SpinBox`))))

(event `SetSkeletalMesh`
  (params (Skeletal :type "SkeletalMesh Object Reference"))
  (`SkeletalMeshComponent.SetSkeletalMeshAsset` (`self.Weapon`) Skeletal))

(fn `BuyBox`
  (params (Player :type "/Game/BP_/Player/BP_Player Object Reference"))
  (if (>= (`/Game/BP_/BP_Component/BPC_Score.Score` (`/Game/BP_/Player/BP_Player.BPC_Score` (`local.Player`))) (`self.Price`))
    (`/Game/BP_/BP_Component/BPC_Score.SubstractServer` (`/Game/BP_/Player/BP_Player.BPC_Score` (`local.Player`)) (`self.Price`))
    (`self.GetWeaponNumber`)))

(fn `GetTextInteract`
  (returns (Text :type Text))
  (if (`self.CanInteract`)
    (return (`self.SetText`))))

(fn `GetWeaponNumber`
  (if (`self.CanInteract`)
    (set `self.CanInteract` false)
    (`KismetArrayLibrary.Array_Clear` (`self.WeaponsList`))
    (bind _outrownames (`DataTableFunctionLibrary.GetDataTableRowNames` "/Game/BP_/Weapons/Enum/DT_Weapons.DT_Weapons"))
    (for _array_element _outrownames
      (bind _returnvalue (`|GetDataTableRow` "/Game/BP_/Weapons/Enum/DT_Weapons.DT_Weapons" _array_element)
        (:`then`
          (`KismetArrayLibrary.Array_Add` (`self.WeaponsList`) _returnvalue)
          (`/Engine/EditorBlueprintResources/StandardMacros.IncrementInt` (`self.RowAmount`)))))
    (`self.OpenCrate`)))

(fn `GetWinerWeapon`
  (locals (TotalWeight :type "Float (double-precision)") (RandomWeight :type "Float (double-precision)"))
  (for _array_element (`self.WeaponsList`)
    (set `local.TotalWeight` (+ (`.ChanceToSpawn_22_E84DC0104EC9960773E39EA7DE02DD96` (break `/Game/BP_/Weapons/Enum/Struct_Weapon` _array_element)) (`local.TotalWeight`))))
  (set `local.RandomWeight` (`KismetMathLibrary.RandomFloatInRange` 0.0 (`local.TotalWeight`)))
  (for _array_element_2 (`self.WeaponsList`)
    (bind _output_get (set `local.RandomWeight` (- (`local.RandomWeight`) (`.ChanceToSpawn_22_E84DC0104EC9960773E39EA7DE02DD96` (break `/Game/BP_/Weapons/Enum/Struct_Weapon` _array_element_2)))))
    (if (<= _output_get 0.0)
      (`self.SetWinerWeaponClient` _array_element_2)
      (break))))

(fn `SetState`
  (set `self.CanInteract` true)
  (set `self.LastWeaponIndex` 0)
  (set `self.RowAmount` 0)
  (set `self.State` "NewEnumerator0")
  (`SkeletalMeshComponent.SetSkeletalMeshAsset` (`self.Weapon`) null)
  (set `self.SpinIndex` 1))

(fn `SetText`
  (returns (Text :type Text))
  (bind _winnerweapon_weaponname (break `/Game/BP_/Weapons/Enum/Struct_Weapon` (`self.WinnerWeapon`)))
  (if (`|EnumEquality` (`self.State`) "NewEnumerator0")
    (set `self.TextInteract` (`KismetTextLibrary.Conv_StringToText` (`KismetStringLibrary.Concat_StrStr` (`KismetTextLibrary.Conv_TextToString` (`self.TextInteraction`)) (`self.NameObejct`) "[Cost: " (`KismetStringLibrary.Conv_IntToString` (`self.Price`)) "]")))
    (else
      (set `self.TextInteract` (`KismetTextLibrary.Conv_StringToText` (`KismetStringLibrary.Concat_StrStr` "Hold E to take " "[ " (`KismetStringLibrary.Conv_NameToString` _winnerweapon_weaponname) "]")))))
  (return (`self.TextInteract`)))

(fn `SetWiner`
  (params (Weapon :type "/Game/BP_/Weapons/Enum/Struct_Weapon Structure"))
  (`SkeletalMeshComponent.SetSkeletalMeshAsset` (`self.Weapon`) Weapon_WeaponSK_18_82D305814B0EFC10FACFBDB9B552FD95)
  (set `self.State` "NewEnumerator1")
  (set `self.CanInteract` true)
  (`self.CloseBoxSlowly`))

(fn `TakeWeapon`
  (params (Player :type "/Game/BP_/Player/BP_Player Object Reference"))
  (bind (_winnerweapon_weaponname _winnerweapon_weaponmesh _winnerweapon_weaponcomponent) (break `/Game/BP_/Weapons/Enum/Struct_Weapon` (`self.WinnerWeapon`)))
  (`|AddComponentByClass` :`self` Player :`Class` _winnerweapon_weaponcomponent)
  (`SkeletalMeshComponent.SetSkeletalMeshAsset` (`self.Weapon`) null)
  (`self.CloseBox`))

(fn `UserConstructionScript`)