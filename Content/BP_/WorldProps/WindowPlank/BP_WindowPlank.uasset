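; Boarded-up window prop whose planks can be removed one by one until vaulting is enabled.
; On BeginPlay it gathers the Window's static mesh children into a shuffled array, then jitters each plank's pitch and position, choosing the offset axis by its orientation.
; GetPlank returns a random remaining plank.
; RemovePlank drops one from the array, switches some collision responses to overlap and sets CanVolting when the count reaches zero.
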(event `self.ReceiveBeginPlay`
  (`self.RandomisePlanksOrder`)
  (`self.RandomisePlanksTransform`))

(fn `GetPlank`
  (returns (Plank :type "StaticMeshComponent Object Reference"))
  (return (`KismetArrayLibrary.Array_Random` (`self.PlanksArray`))))

(fn `RandomisePlanksOrder`
  (bind _planksarray (`self.PlanksArray`))
  (for _array_element (`SceneComponent.GetChildrenComponents` (`self.Window`) false)
    (bind _asstatic_mesh_component (cast `StaticMeshComponent` _array_element))
    (`KismetArrayLibrary.Array_Add` (`self.PlanksArray`) _asstatic_mesh_component))
  (`KismetArrayLibrary.Array_Shuffle` _planksarray)
  (set `self.PlanksNumber` (`KismetArrayLibrary.Array_Length` _planksarray)))

(fn `RandomisePlanksTransform`
  (locals (CurrentPlank :type "SceneComponent Object Reference"))
  (bind _returnvalue (`KismetMathLibrary.RandomFloatInRange` -10.0 10.0))
  (bind (_relativerotation_roll _relativerotation_pitch) (`KismetMathLibrary.BreakRotator` (`SceneComponent.RelativeRotation` (`local.CurrentPlank`))))
  (for _array_element (`self.PlanksArray`)
    (bind _output_get (set `local.CurrentPlank` _array_element))
    (bind _returnvalue_2 (`SceneComponent.GetRelativeTransform` _output_get))
    (`SceneComponent.K2_SetRelativeTransform` (`local.CurrentPlank`) (`KismetMathLibrary.MakeTransform` (+ (.location _returnvalue_2) (`KismetMathLibrary.SelectVector` (`KismetMathLibrary.MakeVector` _returnvalue) (`KismetMathLibrary.MakeVector` 0.0 0.0 _returnvalue) (< _relativerotation_pitch -70.0))) (`KismetMathLibrary.MakeRotator` (.roll (.rotation _returnvalue_2)) (+ (.pitch (.rotation _returnvalue_2)) (`KismetMathLibrary.RandomFloatInRange` -10.0 10.0)) (.yaw (.rotation _returnvalue_2))) (.scale _returnvalue_2)) false false)))

(fn `RemovePlank`
  (params (PlankToRemove :type "StaticMeshComponent Object Reference"))
  (`KismetArrayLibrary.Array_RemoveItem` (`self.PlanksArray`) PlankToRemove)
  (`PrimitiveComponent.SetCollisionResponseToChannel` PlankToRemove "ECC_Pawn" "ECR_Overlap")
  (`PrimitiveComponent.SetCollisionResponseToChannel` PlankToRemove "ECC_PhysicsBody" "ECR_Overlap")
  (`PrimitiveComponent.SetCollisionResponseToChannel` PlankToRemove "ECC_WorldDynamic" "ECR_Overlap")
  (bind _output_get (set `self.PlanksNumber` (`KismetMathLibrary.Clamp` (- (`self.PlanksNumber`) 1) 0 (`self.PlanksNumber`))))
  (if (== _output_get 0)
    (set `self.CanVolting` true)))

(fn `UserConstructionScript`)