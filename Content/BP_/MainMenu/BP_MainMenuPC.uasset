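; Main menu PlayerController that sets up the menu screen and player info for the local player.
; On BeginPlay, Setup shows the cursor, switches to UI-only input, calls SetupPlayerInfo and adds WB_MainMenu to the viewport.
; BeginPlay then loads and saves player data through the GameInstance.
; SetupPlayerInfo and the PlayerInfo RepNotify both pass the controller to BP_MainMenuGM's UpdatePlayerInfo, which requires a valid game mode cast.
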(event `self.ReceiveBeginPlay`
  (bind _returnvalue (`GameplayStatics.GetGameInstance`))
  (`self.Setup`)
  (message `/Game/BP_/Interface/BPI_Saving.LoadPlayerSave` _returnvalue self)
  (message `/Game/BP_/Interface/BPI_Saving.Save` _returnvalue))

(event `SetupPlayerInfo`
  (bind _asbp_main_menu_gm (cast `/Game/BP_/MainMenu/BP_MainMenuGM` (`GameplayStatics.GetGameMode`)))
  (`/Game/BP_/MainMenu/BP_MainMenuGM.UpdatePlayerInfo` _asbp_main_menu_gm self))

(fn `OnRep_PlayerInfo`
  (bind _asbp_main_menu_gm (cast `/Game/BP_/MainMenu/BP_MainMenuGM` (`GameplayStatics.GetGameMode`)))
  (`/Game/BP_/MainMenu/BP_MainMenuGM.UpdatePlayerInfo` _asbp_main_menu_gm self))

(fn `Setup`
  (if (`self.IsLocalPlayerController`)
    (set `self.bShowMouseCursor` true)
    (`WidgetBlueprintLibrary.SetInputMode_UIOnlyEx` self null)
    (`self.SetupPlayerInfo`)
    (bind _returnvalue (`|CreateWidget` "/Game/BP_/MainMenu/Widget/WB_MainMenu.WB_MainMenu_C"))
    (bind _output_get (set `self.MainMenu` _returnvalue))
    (`UserWidget.AddToViewport` _output_get 0)))

(fn `UserConstructionScript`)