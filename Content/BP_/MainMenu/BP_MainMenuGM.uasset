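; BP_MainMenuGM is the main menu game mode, which passes a player's profile info to the game instance.
; UpdatePlayerInfo stores the requesting controller and builds an SMainPlayerInfo struct from its name, player state, and the XP and level held on BP_MainMenuPC.
; It sends that struct through a SetPlayerInfo message call, so it needs no cast to a specific game instance class.
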(fn `UpdatePlayerInfo`
  (params (RequestingPC :type "PlayerController Object Reference"))
  (locals (PlayerController :type "PlayerController Object Reference"))
  (bind _requestingpc (`local.RequestingPC`))
  (bind (_playerinfo_playercontroller _playerinfo_playername _playerinfo_playerstate _playerinfo_xp _playerinfo_level) (break `/Game/BP_/MainMenu/S_MainPlayerInfo` (`/Game/BP_/MainMenu/BP_MainMenuPC.PlayerInfo` (cast `/Game/BP_/MainMenu/BP_MainMenuPC` _requestingpc :!pure true))))
  (set `local.PlayerController` RequestingPC)
  (message `/Game/BP_/Interface/BPI_GameInstance.SetPlayerInfo` (`GameplayStatics.GetGameInstance`) (make `/Game/BP_/MainMenu/S_MainPlayerInfo` (`local.RequestingPC`) (`KismetTextLibrary.Conv_StringToText` (`AdvancedSessionsLibrary.GetPlayerName` _requestingpc)) (`Controller.PlayerState` _requestingpc) _playerinfo_xp _playerinfo_level))
  (return))

(fn `UserConstructionScript`)