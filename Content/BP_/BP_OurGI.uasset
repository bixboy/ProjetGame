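; BP_OurGI, apparently the Game Instance, provides events to host and join multiplayer sessions through Advanced Sessions nodes.
; CreatSession creates a four-connection session and, on success, opens the lobby level as a listen server.
; FindSession searches all server types, joins the first result without checking for an empty list, and records the outcome in SuccessJoiningSession with debug prints.
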(event `CreatSession`
  (`CreateSessionCallbackProxyAdvanced.CreateAdvancedSession` :`PlayerController` (`GameplayStatics.GetPlayerController` 0) :`PublicConnections` 4
    (:`OnSuccess`
      (`GameplayStatics.OpenLevelBySoftObjectPtr` "/Game/level/Lvl_Lobby.Lvl_Lobby" true "listen"))))

(event `FindSession`
  (bind _results (`FindSessionsCallbackProxyAdvanced.FindSessionsAdvanced` (`GameplayStatics.GetPlayerController` 0) 0 false "AllServers")
    (:`OnSuccess`
      (`KismetSystemLibrary.PrintString` "Find Session")
      (`JoinSessionCallbackProxy.JoinSession` (`GameplayStatics.GetPlayerController` 0) (`|GetArrayItem` _results)
        (:`OnSuccess`
          (`KismetSystemLibrary.PrintString` "Join session")
          (set `self.SuccessJoiningSession` true))
        (:`OnFailure`
          (`KismetSystemLibrary.PrintString` "Failed to join session")
          (set `self.SuccessJoiningSession` false))))
    (:`OnFailure`
      (`KismetSystemLibrary.PrintString` "Failed to join session")
      (set `self.SuccessJoiningSession` false))))